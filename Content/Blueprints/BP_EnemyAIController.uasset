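; AI controller that makes a BP_EnemyCharacter flee whenever the player enters its FleeRadius.
; Each tick builds five candidate ray endpoints: one directly away from the player, plus yaw-rotated copies of that world position (not of the direction).
; Flee line-traces toward them, moves to the hit location with the greatest distance, then re-checks on arrival or failure.
; Tick also restarts idle fleeing and draws debug shapes; simpler BasicFlee is unused.
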(event Custom|BasicFlee
  (bind _returnvalue (Game|GetPlayerCharacter 0))
  (bind _controlledenemy (Variables|EnemyInfo|GetControlledEnemy))
  (bind _currentenemylocation (Variables|EnemyInfo|GetCurrentEnemyLocation))
  (bind _fleeradius (Variables|/Game/Blueprints/BP_EnemyCharacter.BP_EnemyCharacter_C|GetFleeRadius _controlledenemy))
  ;[1 1 1] Basic Flee Behaviour; will work but will easily get stuck on corners etc
  ;;[1 1 1] Check if Player is within the flee radius
  (if (<= (Transformation|GetDistanceTo _returnvalue _controlledenemy) _fleeradius)
    (AI|AIMoveTo 0 (+ _currentenemylocation (* (Math|Vector|Normalize (- _currentenemylocation (Transformation|GetActorLocation _returnvalue))) _fleeradius)) 0 5.0 false
      (:OnSuccess
        _)
      (:OnFail
        _))
    (CallFunction|BasicFlee)
    (else
      (AI|Navigation|StopMovement))))

(event Custom|Flee
  (bind _controlledenemy (Variables|EnemyInfo|GetControlledEnemy))
  ;[1 1 1] Check if Player is within the flee radius, only then we run away
  (if (<= (Transformation|GetDistanceTo (Game|GetPlayerCharacter 0) _controlledenemy) (Variables|/Game/Blueprints/BP_EnemyCharacter.BP_EnemyCharacter_C|GetFleeRadius _controlledenemy))
    (Variables|EnemyInfo|SetHasArrived false)
    ;[1 1 1] For safety, add our Enemy as actor to ignore
    (Variables|RayCastInfo|SetActorsToIgnore (Utilities|Array|MakeArray (Variables|EnemyInfo|GetControlledEnemy)))
    ;[1 1 1] Check each direction
    (for _array_element (Variables|RayCastInfo|GetDirectionsToCheck)
      ;[1 1 1] Execute and store all possible locations with their distances
      (bind (_distance _location) (CallFunction|RayTraceDirections (Variables|EnemyInfo|GetCurrentEnemyLocation) _array_element (Variables|RayCastInfo|GetActorsToIgnore)))
      (Utilities|FlowControl|Sequence
        (:then_0
          (Utilities|Array|Add (Variables|RayCastOut|GetRayCastHitDistances) _distance))
        (:then_1
          (Utilities|Array|Add (Variables|RayCastOut|GetRayCastHitLocations) _location))))
    ;[1 1 1] Get the location that is furthest away
    (bind _output_get (Variables|EnemyInfo|SetEnemyDestination (Utilities|Array|Get(acopy) (Variables|RayCastOut|GetRayCastHitLocations) (.IndexOfMaxValue (Math|Float|MaxOfFloatArray (Variables|RayCastOut|GetRayCastHitDistances))))))
    ;[1 1 1] Move to that location
    (AI|AIMoveTo (Variables|EnemyInfo|GetControlledEnemy) _output_get 0 -1.0 false
      (:OnSuccess
        _)
      (:OnFail
        _))
    ;[1 1 1] Cleanup
    (Variables|EnemyInfo|SetHasArrived true)
    (Utilities|Array|Clear (Variables|RayCastOut|GetRayCastHitDistances))
    (Utilities|Array|Clear (Variables|RayCastOut|GetRayCastHitLocations))
    ;[1 1 1] Check if player isn't in radius anymore
    (CallFunction|Flee)
    (else
      (AI|Navigation|StopMovement))))

(event EventBeginPlay
  ;[1 1 1] Check if the current pawn is an EnemyCharacter
  (bind _asbp_enemy_character (Utilities|Casting|CastToBP_EnemyCharacter (Pawn|GetControlledPawn)))
  (bind _output_get (Variables|EnemyInfo|SetControlledEnemy _asbp_enemy_character))
  ;[1 1 1] Get its location and start Fleeing if needed
  (Variables|EnemyInfo|SetCurrentEnemyLocation (Transformation|GetActorLocation _output_get))
  (CallFunction|Flee))

(event EventTick
  (params (DeltaSeconds :type Float%20%28single-precision%29))
  (bind _controlledenemy (Variables|EnemyInfo|GetControlledEnemy))
  (bind _controlledenemy_2 (Variables|EnemyInfo|GetControlledEnemy))
  ;[1 1 1] Cache our enemy location
  (bind _output_get (Variables|EnemyInfo|SetCurrentEnemyLocation (Transformation|GetActorLocation _controlledenemy_2)))
  (Rendering|Debug|DrawDebugSphere _output_get (Variables|/Game/Blueprints/BP_EnemyCharacter.BP_EnemyCharacter_C|GetFleeRadius _controlledenemy_2) 12 "(R=1.000000,G=0.015625,B=0.015625,A=1.000000)" 0.0 2.0)
  ;[1 1 1] Calculate all the directions we need to check
  (bind _array (CallFunction|GetAllDirectionstoCheck))
  (Variables|RayCastInfo|SetDirectionsToCheck _array)
  (Utilities|FlowControl|Sequence
    (:then_0
      ;[1 1 1] If needed, start Flee
      (if (and (Variables|EnemyInfo|GetHasArrived) (<= (Transformation|GetDistanceTo (Game|GetPlayerCharacter 0) _controlledenemy) (Variables|/Game/Blueprints/BP_EnemyCharacter.BP_EnemyCharacter_C|GetFleeRadius _controlledenemy)))
        (CallFunction|Flee)))
    (:then_1
      ;[1 1 1] Draw Debug
      (for _array_element (Variables|RayCastInfo|GetDirectionsToCheck)
        (Rendering|Debug|DrawDebugLine (Variables|EnemyInfo|GetCurrentEnemyLocation) _array_element "(R=1.000000,G=0.017018,B=0.831713,A=1.000000)" 0.0 1e+01))
      (Rendering|Debug|DrawDebugLine (Variables|EnemyInfo|GetCurrentEnemyLocation) (Variables|EnemyInfo|GetEnemyDestination) "(R=0.057249,G=1.000000,B=0.000000,A=1.000000)" 0.0 1e+01))))

(fn ConstructionScript)

(fn RayTraceDirections
  (params (Start :type Vector) (End :type Vector) (ActorsToIgnore :type Array%20of%20Actor%20Object%20References))
  (bind _outhit (Collision|LineTraceByChannel Start End "TraceTypeQuery1" false ActorsToIgnore "None"))
  (return (.Distance (Collision|BreakHitResult _outhit)) (.Location (Collision|BreakHitResult _outhit))))

(fn GetAllDirectionstoCheck
  (bind _returnvalue (Game|GetPlayerCharacter 0))
  (bind _minimumraylength (Variables|RayCastInfo|GetMinimumRayLength))
  (bind _currentenemylocation (Variables|EnemyInfo|GetCurrentEnemyLocation))
  (bind _returnvalue_2 (Transformation|GetActorLocation _returnvalue))
  (bind _returnvalue_3 (- _currentenemylocation _returnvalue_2))
  (bind _returnvalue_4 (Math|Vector|Normalize _returnvalue_3))
  (bind _returnvalue_5 (* _returnvalue_4 _minimumraylength))
  (bind _returnvalue_6 (+ _currentenemylocation _returnvalue_5))
  ;[1 1 1] Add all directions that we want to check to an array
  (return (Utilities|Array|MakeArray _returnvalue_6 (Math|Vector|RotateVector _returnvalue_6 "0,75.000000,0.000000") (Math|Vector|RotateVector _returnvalue_6 "0.000000,-75.000000, 0") (Math|Vector|RotateVector _returnvalue_6 "0,110.000000, 0") (Math|Vector|RotateVector _returnvalue_6 "0,-110.000000, 0"))))
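; BP_EnemyCharacter is a mouse that the player catches or that gets held by placed mouse traps.
; Overlapping a placed, empty trap deactivates its movement and notifies the trap; ending overlap with any trap reactivates movement.
; Overlapping the player reports the mouse's value, plays a pickup sound and destroys the mouse.
; The non-looping Squeek audio replays whenever it finishes, with the cue delaying each start.
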(event OnAudioFinished(Squeek)
  ;[1 1 1] Our sound cue isn't looping, when it has finished playing, play again, the start will be delayed again
  (Audio|Components|Audio|Play (Variables|Default|GetSqueek) 0.0))

(event EventBeginPlay
  (|CallParentFunction) ; This node is disabled and will not be called.\nDrag off pins to build functionality.
)

(event Collision|EventActorEndOverlap
  (params (OtherActor :type Actor%20Object%20Reference))
  ;[1 1 1] When the trap despawns, we are free to move again
  (Utilities|Casting|CastToBP_MouseTrap OtherActor)
  (Components|Activation|Activate (Variables|Character|GetCharacterMovement) false))

(event EventTick
  (params (DeltaSeconds :type Float%20%28single-precision%29))
  (|CallParentFunction DeltaSeconds) ; This node is disabled and will not be called.\nDrag off pins to build functionality.
)

(event Collision|EventActorBeginOverlap
  (params (OtherActor :type Actor%20Object%20Reference))
  (Utilities|FlowControl|Sequence
    (:then_0
      ;[1 1 1] If we overlap with a placed trap that hasn't caught a mouse yet, we stop moving
      (bind _asbp_mouse_trap (Utilities|Casting|CastToBP_MouseTrap OtherActor))
      (if (Variables|/Game/Blueprints/BP_MouseTrap.BP_MouseTrap_C|GetIsPlaced _asbp_mouse_trap)
        (if (not (Variables|/Game/Blueprints/BP_MouseTrap.BP_MouseTrap_C|GetHasCaughtMouse _asbp_mouse_trap))
          (Components|Activation|Deactivate (Variables|Character|GetCharacterMovement))
          (Default|CaughtMouse _asbp_mouse_trap))))
    (:then_1
      ;[1 1 1] If we hit a player, play death sound and destroy actor
      (bind _asbp_player_character (Utilities|Casting|CastToBP_PlayerCharacter OtherActor))
      (Default|CaughtAMouse _asbp_player_character (Variables|Default|GetMouseValue))
      (Audio|PlaySoundatLocation "/Game/Audio/Pickup_Sound.Pickup_Sound" (Transformation|GetActorLocation) "0, 0, 0" 1.0 1.0 0.0 0 0 0)
      (Actor|DestroyActor))))

(fn ConstructionScript
  (|CallParentFunction))
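; BP_RouteBlocker is an obstacle the player triggers once with E within a radius to block a route.
; It starts passable, then swaps the inactive mesh for the active one, enables collision and plays a drop sound.
; Blocking also sets the NavModifier to NavArea_Null to break the navmesh and enables an invisible-to-movement-until-then wall that stops mouse Visibility traces.
; Tick draws the trigger radius as a debug sphere.
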(event Custom|StartBlocking
  (bind _block_active (Variables|Default|GetBlock_Active))
  (bind _block_active_rayblockelement (Variables|Default|GetBlock_Active_RayBlockElement))
  ;[1 1 1] Change Visibility
  (Rendering|SetVisibility (Variables|Default|GetBlock_Inactive) false true)
  (Rendering|SetVisibility _block_active true true)
  ;[1 1 1] Enable Collision on the cylinder laying down
  (Collision|SetCollisionEnabled _block_active "QueryAndPhysics")
  ;[1 1 1] This is a wall that will block raycasts from the mice, update the collision preset
  (Collision|SetCollisionResponsetoChannel _block_active_rayblockelement "ECC_Visibility" "ECR_Block")
  (Collision|SetCollisionEnabled _block_active_rayblockelement "QueryAndPhysics")
  ;[1 1 1] Make Sure the Nav Modifier breaks the navmesh
  (Class|NavModifierComponent|SetAreaClass (Variables|Default|GetNavModifier) "/Script/NavigationSystem.NavArea_Null")
  ;[1 1 1] Play Sound
  (Audio|SpawnSoundatLocation "/Game/Audio/PathBlockDrop.PathBlockDrop" (Transformation|GetActorLocation) "0, 0, 0" 1.0 1.0 0.0 0 0))

(event EventBeginPlay
  (bind _block_active_rayblockelement (Variables|Default|GetBlock_Active_RayBlockElement))
  ;[1 1 1] In the beginning, the route isn't blocked yet, so don't change the navmesh, hide the BlockActive Meshesh
  (Class|NavModifierComponent|SetAreaClass (Variables|Default|GetNavModifier) "/Script/NavigationSystem.NavArea")
  (Rendering|SetVisibility (Variables|Default|GetBlock_Active) false false)
  ;[1 1 1] We Start our Wall with BlockAllDynamic, otherwise this will generate problems later, but we want to be able to move through it. Change those properties first
  (Collision|SetCollisionResponsetoChannel _block_active_rayblockelement "ECC_Visibility" "ECR_Ignore")
  (Collision|SetCollisionEnabled _block_active_rayblockelement "NoCollision"))

(event Collision|EventActorBeginOverlap
  (params (OtherActor :type Actor%20Object%20Reference)))

(event EventTick
  (params (DeltaSeconds :type Float%20%28single-precision%29))
  ;[1 1 1] Purely Debug Draw
  (Rendering|Debug|DrawDebugSphere (Transformation|GetActorLocation) (Variables|Default|GetRadius) 12 "(R=1.000000,G=0.015625,B=0.015625,A=1.000000)" 0.0 2.0))

(event Input|KeyboardEvents|E
  (params (Key :type Key%20Structure :default "None"))
  ;[1 1 1] When Player is close enough and pressed "e". start blocking the path
  (:Released
    (if (not (Variables|Default|GetIsBlockActive))
      (bind _asbp_player_character (Utilities|Casting|CastToBP_PlayerCharacter (Game|GetPlayerCharacter 0)))
      (if (<= (Transformation|GetDistanceTo _asbp_player_character) (Variables|Default|GetRadius))
        (CallFunction|StartBlocking)
        (Variables|Default|SetIsBlockActive true)))))

(fn ConstructionScript)
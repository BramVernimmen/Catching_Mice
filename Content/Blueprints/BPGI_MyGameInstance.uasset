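; Game instance that tracks the current level index and handles level progression and reloading.
; LoadNextLevel advances the index through the LevelNames array and opens that level by name, replaying the last one once the end is reached.
; ReloadLevel reopens the level at the current index.
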(event Custom|LoadNextLevel
  ;[1 1 1] If the index isn't the final index to access a level; increment it and load the next level, else loop the last level
  (if (== (+ (Variables|Default|GetLevelIndex) 1) (Utilities|Array|Length (Variables|Default|GetLevelNames)))
    _
    (else
      (Math|Integer|IncrementInt (Variables|Default|GetLevelIndex)
        (:%20%20
          _))))
  (Game|OpenLevel(byName) (Utilities|Array|Get(acopy) (Variables|Default|GetLevelNames) (Variables|Default|GetLevelIndex))))

(event Custom|Reload%20Level
  ;[1 1 1] Reload Current Level
  (Game|OpenLevel(byName) (Utilities|Array|Get(acopy) (Variables|Default|GetLevelNames) (Variables|Default|GetLevelIndex))))
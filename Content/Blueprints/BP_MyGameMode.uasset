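; Game mode that runs a timed level where all enemies must be eliminated before the countdown expires.
; On BeginPlay it caches all enemies and the player, then sets the timer component's max time in proportion to enemy count.
; Tick marks the level completed when no valid enemies remain, otherwise advances the countdown; timeout also completes it and triggers the player's loss.
; Events expose toggling the timer and adding extra time.
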(event OnTimeIsUp(BPC_Timer)
  ;[1 1 1] When Time is up, set level to Completed and Trigger loss screen
  (Variables|Default|SetIsLevelCompleted true)
  (Default|TriggerLoss (Variables|Default|GetPlayerCharacter)))

(event OnTimeIsUp(Timer)
  ;[1 1 1] When Time is up, set level to Completed and Trigger loss screen
  (Variables|Default|SetIsLevelCompleted true)
  (Default|TriggerLoss (Variables|Default|GetPlayerCharacter)))

(event Custom|Change%20Timer%20State
  ;[1 1 1] Turning the timer on/off
  (Class|TimerComponent|ChangeActiveState (Variables|Default|GetTimer)))

(event Custom|AddExtraTime
  (params (extraTimeToAdd :type Float%20%28single-precision%29))
  ;[1 1 1] Add Extra Time to the Timer (We cap at MaxTime)
  (Class|TimerComponent|AddTime (Variables|Default|GetTimer) extraTimeToAdd))

(event EventBeginPlay
  (bind _returnvalue (Game|GetPlayerCharacter 0))
  (bind _timer (Variables|Default|GetTimer))
  ;[1 1 1] Calculate and set the Max Time for current Level
  (bind _outactors (Actor|GetAllActorsOfClass "/Game/Blueprints/BP_EnemyCharacter.BP_EnemyCharacter_C"))
  (bind _output_get (Variables|Enemies|SetAllEnemies _outactors))
  (bind _output_get_2 (Variables|Enemies|SetMaxAmountOfEnemies (Utilities|Array|Length _output_get)))
  (Variables|/Script/Assignment.TimerComponent|SetMaxTime _timer (* _output_get_2 12.5))
  (Class|TimerComponent|ResetTimer _timer)
  ;[1 1 1] Cache our Player Character
  (Utilities|IsValid _returnvalue
    (:Is%20Valid
      (bind _asbp_player_character (Utilities|Casting|CastToBP_PlayerCharacter _returnvalue))
      (Variables|Default|SetPlayerCharacter _asbp_player_character))))

(event EventTick
  (params (DeltaSeconds :type Float%20%28single-precision%29))
  (if (not (Variables|Default|GetIsLevelCompleted))
    (Utilities|FlowControl|Sequence
      (:then_0
        ;[1 1 1] Check how many Enemies are left alive, if none are, we set our Level to Completed
        (Variables|Enemies|SetEnemiesLeft 0)
        (for _array_element (Variables|Enemies|GetAllEnemies)
          (Utilities|IsValid _array_element
            (:Is%20Valid
              (Math|Integer|IncrementInt (Variables|Enemies|GetEnemiesLeft)))))
        (if (== (Variables|Enemies|GetEnemiesLeft) 0)
          (Variables|Default|SetIsLevelCompleted true)))
      (:then_1
        ;[1 1 1] Check again if our level is completed, this might've changed in the first Sequence hit
        (if (not (Variables|Default|GetIsLevelCompleted))
          ;[1 1 1] Count Down the Timer
          (Class|TimerComponent|DoCountDown (Variables|Default|GetTimer) DeltaSeconds))))))

(fn ConstructionScript)
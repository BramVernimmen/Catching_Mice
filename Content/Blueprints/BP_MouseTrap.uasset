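; BP_MouseTrap is a mouse trap actor that exists either as a dropped, spinning item or as a placed trap.
; PlaceTrap sets it placed, swaps the dropped mesh for the placed one and turns off the particles.
; CaughtMouse flags the catch, plays a sound and changes the trap's material.
; Tick then runs the Timer countdown, whose OnTimeIsUp event destroys the trap with a breaking sound.
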(event OnTimeIsUp(Timer)
  ;[1 1 1] When time is up, destroy the trap, play a sound
  (Actor|DestroyActor)
  (Audio|PlaySoundatLocation "/Game/Audio/Mouse_Trap_Broken.Mouse_Trap_Broken" (Transformation|GetActorLocation) "0, 0, 0" 1.0 1.0 0.0 0 0 0))

(event Custom|PlaceTrap
  ;[1 1 1] This Event will make the trap active and visible
  (Variables|Default|SetIsPlaced true)
  ;[1 1 1] Check what type of Mesh should be visible
  (if (Variables|Default|GetIsPlaced)
    ;[1 1 1] Switching the visibility
    (Rendering|SetVisibility (Variables|Default|GetDroppedTrap) false false)
    (Rendering|SetVisibility (Variables|Default|GetPlacedTrap) true false)
    ;[1 1 1] We only want to see the particles when it's dropped
    (Components|Activation|Deactivate (Variables|Default|GetParticleSystem))
    (else
      (Rendering|SetVisibility (Variables|Default|GetPlacedTrap) false false)
      (Rendering|SetVisibility (Variables|Default|GetDroppedTrap) true false))))

(event Custom|CaughtMouse
  ;[1 1 1] When we caught a mouse, we remember this, play a sound, and change the color
  (Variables|Default|SetHasCaughtMouse true)
  (Audio|PlaySoundatLocation "/Game/Audio/Mouse_Trap.Mouse_Trap" (Transformation|GetActorLocation) "0, 0, 0" 1.0 1.0 0.0 0 0 0)
  (Rendering|Material|SetMaterial (Variables|Default|GetPlacedTrap) 0 "/Game/Materials/MAT_TrapCaughtColor.MAT_TrapCaughtColor"))

(event EventBeginPlay
  ;[1 1 1] Check what type of Mesh should be visible
  (if (Variables|Default|GetIsPlaced)
    ;[1 1 1] Switching the visibility
    (Rendering|SetVisibility (Variables|Default|GetDroppedTrap) false false)
    (Rendering|SetVisibility (Variables|Default|GetPlacedTrap) true false)
    ;[1 1 1] We only want to see the particles when it's dropped
    (Components|Activation|Deactivate (Variables|Default|GetParticleSystem))
    (else
      (Rendering|SetVisibility (Variables|Default|GetPlacedTrap) false false)
      (Rendering|SetVisibility (Variables|Default|GetDroppedTrap) true false))))

(event Collision|EventActorBeginOverlap
  (params (OtherActor :type Actor%20Object%20Reference)))

(event EventTick
  (params (DeltaSeconds :type Float%20%28single-precision%29))
  (if (Variables|Default|GetIsPlaced)
    ;[1 1 1] Only count down when we caught a mouse
    (if (Variables|Default|GetHasCaughtMouse)
      (Class|TimerComponent|DoCountDown (Variables|Default|GetTimer) DeltaSeconds))
    (else
      ;[1 1 1] When the trap isn't placed, rotate it to make it look more appealing
      (Transformation|AddActorLocalRotation "0,2.000000, 0" false false))))

(fn ConstructionScript)
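; Player controller that moves the controlled pawn along fixed world X and Y axes from the forward and right input axes.
; Both axis events cast the game mode to BP_MyGameMode and ignore input once the level is completed.
; After adding movement, both share logic that turns the control rotation toward the last movement input vector, keeping yaw and roll but zeroing pitch.
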(event EventBeginPlay)

(event EventTick
  (params (DeltaSeconds :type Float%20%28single-precision%29)))

(event Input|AxisEvents|InputAxisMovementForward
  (params (AxisValue :type Float%20%28single-precision%29))
  (bind _returnvalue (Pawn|GetControlledPawn))
  (bind _returnvalue_2 (Class|Pawn|GetLastMovementInputVector _returnvalue))
  (bind _returnvalue_3 (Math|Conversions|RotationFromXVector _returnvalue_2))
  ;[1 1 1] Handle movement when the Level hasn't been Completed yet
  (bind _asbp_my_game_mode (Utilities|Casting|CastToBP_MyGameMode (Game|GetGameMode)))
  (if (not (Variables|/Game/Blueprints/BP_MyGameMode.BP_MyGameMode_C|GetIsLevelCompleted _asbp_my_game_mode))
    (Pawn|Input|AddMovementInput _returnvalue "1.000000, 0, 0" AxisValue false)
    ;[1 1 1] Handle Rotation of Player Character
    (if (> (Math|Vector|VectorLength _returnvalue_2) 0.0)
      (Pawn|SetControlRotation (Math|Rotator|MakeRotator (.roll _returnvalue_3) 0.0 (.yaw _returnvalue_3))))))

(event Input|AxisEvents|InputAxisMovementRight
  (params (AxisValue :type Float%20%28single-precision%29))
  (bind _returnvalue (Pawn|GetControlledPawn))
  (bind _returnvalue_2 (Class|Pawn|GetLastMovementInputVector _returnvalue))
  (bind _returnvalue_3 (Math|Conversions|RotationFromXVector _returnvalue_2))
  ;[1 1 1] Handle movement when the Level hasn't been Completed yet
  (bind _asbp_my_game_mode (Utilities|Casting|CastToBP_MyGameMode (Game|GetGameMode)))
  (if (not (Variables|/Game/Blueprints/BP_MyGameMode.BP_MyGameMode_C|GetIsLevelCompleted _asbp_my_game_mode))
    (Pawn|Input|AddMovementInput _returnvalue "0,1.000000, 0" AxisValue false)
    ;[1 1 1] Handle Rotation of Player Character
    (if (> (Math|Vector|VectorLength _returnvalue_2) 0.0)
      (Pawn|SetControlRotation (Math|Rotator|MakeRotator (.roll _returnvalue_3) 0.0 (.yaw _returnvalue_3))))))

(fn ConstructionScript)
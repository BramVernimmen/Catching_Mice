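; BPC_Timer is a timer component that holds a current time, filled to its maximum on BeginPlay or ResetTimer.
; It does not tick itself: callers pass an amount to DoCountDown, which subtracts it, clamped between zero and the maximum.
; The OnTimeIsUp dispatcher fires only when a decrease lands on zero, so repeated calls at zero stay silent.
; Helper functions report the fraction remaining and whether time is up.
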(event Custom|ResetTimer
  (Variables|Default|SetCurrentTime (Variables|Default|GetMaxTime)))

(event EventBeginPlay
  (CallFunction|ResetTimer))

(event EventTick
  (params (DeltaSeconds :type Float%20%28single-precision%29)))

(fn GetTimeLeftPercentage
  (return (/ (Variables|Default|GetCurrentTime) (Variables|Default|GetMaxTime))))

(fn IsTimeUp
  (return (== (CallFunction|GetTimeLeftPercentage) 0.0)))

(fn DoCountDown
  (params (Amount :type Float%20%28single-precision%29))
  (bind _istimeup (CallFunction|IsTimeUp))
  ;[1 1 1] Cache original time value
  (LocalVariables|SetOriginalTime (Variables|Default|GetCurrentTime))
  (bind _output_get (Variables|Default|SetCurrentTime (Math|Float|Clamp(Float) (- (Variables|Default|GetCurrentTime) Amount) 0.0 (Variables|Default|GetMaxTime))))
  (if (and _istimeup (> (LocalVariables|GetOriginalTime) _output_get))
    (Default|CallOnTimeIsUp))
  (return _istimeup))
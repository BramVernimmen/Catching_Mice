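; Player character for a mouse-catching game that carries one mouse trap at a time and owns the game HUD.
; Overlapping an unplaced trap picks it up and destroys it; releasing Space spawns and places a new one at ground level, offset by the capsule half-height.
; Mouse catches add time through the game mode, and pickups, placements, catches and level failure update the HUD widget created on BeginPlay.
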(event Custom|Caught%20A%20Mouse
  (params (MouseTimeValue :type Float%20%28single-precision%29))
  ;[1 1 1] When we caught a Mouse, display this to the screen and add extra time to the timer
  (bind _asbp_my_game_mode (Utilities|Casting|CastToBP_MyGameMode (Game|GetGameMode)))
  (Default|AddExtraTime _asbp_my_game_mode MouseTimeValue)
  (Default|MouseCaught (Variables|Default|GetGameHud)))

(event Custom|TriggerLoss
  ;[1 1 1] Trigger Level Failed Menu on HUD
  (Default|LevelFailedMenu (Variables|Default|GetGameHud)))

(event EventBeginPlay
  (|CallParentFunction)
  ;[1 1 1] Create and cache our HUD
  (bind _returnvalue (UserInterface|CreateWidget "/Game/Blueprints/BPW_GameHud.BPW_GameHud_C"))
  (bind _output_get (Variables|Default|SetGameHud _returnvalue))
  (UserInterface|Viewport|AddtoViewport _output_get 0))

(event Collision|EventActorBeginOverlap
  (params (OtherActor :type Actor%20Object%20Reference))
  (|CallParentFunction OtherActor)
  (bind _asbp_mouse_trap (Utilities|Casting|CastToBP_MouseTrap OtherActor))
  ;[1 1 1] Check if the trap is not placed and we have none in our inventory; if true add it to inventory and destroy the old one
  (if (not (Variables|/Game/Blueprints/BP_MouseTrap.BP_MouseTrap_C|GetIsPlaced _asbp_mouse_trap))
    (if (not (Variables|Default|GetHasTrapInInventory))
      (Variables|Default|SetHasTrapInInventory true)
      (Actor|DestroyActor _asbp_mouse_trap)
      ;[1 1 1] Play a picked up sound effect and show on screen that you picked it up/ how to use
      (Audio|PlaySoundatLocation "/Game/Audio/Pickup_Sound.Pickup_Sound" (Transformation|GetActorLocation) "0, 0, 0" 1.0 1.0 0.0 0 0 0)
      (Default|HasTrapinInv (Variables|Default|GetGameHud)))))

(event EventTick
  (params (DeltaSeconds :type Float%20%28single-precision%29))
  (|CallParentFunction DeltaSeconds) ; This node is disabled and will not be called.\nDrag off pins to build functionality.
)

(event Input|KeyboardEvents|SpaceBar
  (params (Key :type Key%20Structure :default "None"))
  (bind _returnvalue (Transformation|GetActorTransform))
  ;[1 1 1] Spawn trap when Space Bar is pressed
  (:Released
    ;[1 1 1] We can only carry 1 trap, so check if we have one
    (if (Variables|Default|GetHasTrapInInventory)
      ;[1 1 1] Spawn the trap
      (bind _returnvalue_2 (Game|SpawnActorfromClass "/Game/Blueprints/BP_MouseTrap.BP_MouseTrap_C" (Math|Transform|MakeTransform (Math|Vector|MakeVector (.x (.location _returnvalue)) (.y (.location _returnvalue)) (- (.z (.location _returnvalue)) (Components|Capsule|GetScaledCapsuleHalfHeight (Variables|Default|GetCapsuleComponent)))) (.rotation _returnvalue) (.scale _returnvalue)) "Undefined" 0 0))
      (Default|PlaceTrap _returnvalue_2)
      ;[1 1 1] Remove the trap from inventory, and hud; play sound of placing trap
      (Variables|Default|SetHasTrapInInventory false)
      (Default|TrapRemovedfromInv (Variables|Default|GetGameHud))
      (Audio|PlaySoundatLocation "/Game/Audio/Trap_Placing.Trap_Placing" (Transformation|GetActorLocation) "0, 0, 0" 1.0 1.0 0.0 0 0 0))))

(fn ConstructionScript
  (|CallParentFunction))